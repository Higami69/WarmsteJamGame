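; BP_Planet_Base is a planet actor that answers gravity and look-alignment queries for a given position.
; CheckGravity returns a pull strength that falls linearly from GravityMaxStrength at the mesh's location to zero at GravityRadius.
; CheckAngularProx returns a score that rises to one as a look direction lines up with the planet's root, and is zero beyond the MinimumAngularProx angle in degrees.
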(fn `CheckAngularProx`
  (params (SourcePos :type "Vector Structure") (LookDir :type "Vector Structure"))
  (returns (SoundRate :type "Float (double-precision)"))
  (bind _minimumangularprox (`self.MinimumAngularProx`))
  (return (/ (`KismetMathLibrary.FMax` (- _minimumangularprox (`KismetMathLibrary.DegAcos` (`KismetMathLibrary.Dot_VectorVector` (`KismetMathLibrary.Normal` (- (`SceneComponent.K2_GetComponentLocation` (`self.DefaultSceneRoot`)) SourcePos)) (`KismetMathLibrary.Normal` LookDir))))) _minimumangularprox)))

(fn `CheckGravity`
  (params (Position :type "Vector Structure"))
  (returns (GravityStrength :type "Float (double-precision)"))
  (bind _gravityradius (`self.GravityRadius`))
  (bind _returnvalue (`KismetMathLibrary.Vector_Distance` Position (`SceneComponent.K2_GetComponentLocation` (`self.StaticMesh`))))
  (if (< _returnvalue _gravityradius)
    (return (* (- 1.0 (/ _returnvalue _gravityradius)) (`self.GravityMaxStrength`)))
    (else
      (return 0.0))))

(fn `UserConstructionScript`)