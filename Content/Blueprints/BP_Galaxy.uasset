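; BP_Galaxy procedurally builds a play space on BeginPlay, spawning one sun and PlanetAmt randomly typed planets within a Size-wide cube around world origin.
; Planet positions use rejection sampling, re-rolling until far enough from the sun and other planets.
; GetSoftCapSpeedMod provides a soft boundary: beyond Size from the actor, outward movement gets a multiplier based on overshoot and heading, while inward movement keeps full speed.
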(event `self.ReceiveBeginPlay`
  (bind _size (`self.Size`))
  (bind _returnvalue (* _size -0.5))
  (bind _returnvalue_2 (* _size 0.5))
  (`|ExecutionSequence`
    (:`then_0`
      (bind _returnvalue_3 (`|SpawnActorFromClass` "/Game/Blueprints/BP_Sun.BP_Sun_C" (`KismetMathLibrary.MakeTransform` (`KismetMathLibrary.MakeVector` (`KismetMathLibrary.RandomFloatInRange` _returnvalue _returnvalue_2) (`KismetMathLibrary.RandomFloatInRange` _returnvalue _returnvalue_2) (`KismetMathLibrary.RandomFloatInRange` _returnvalue _returnvalue_2))) "Undefined" "OverrideRootScale" null null))
      (set `self.Sun` _returnvalue_3))
    (:`then_1`
      ;[1 1 1] Spawn all planets
      (for _ (range (`self.PlanetAmt`))
        (bind _newplanet (`self.SpawnPlanet`))
        (`KismetArrayLibrary.Array_Add` (`self.Objects`) _newplanet)))))

(fn `CheckNewPlanetLocation`
  (params (NewLoc :type "Vector Structure"))
  (returns (IsOkay :type Boolean))
  (if (> (`KismetMathLibrary.Vector_Distance` NewLoc (`SceneComponent.K2_GetComponentLocation` (`/Game/Blueprints/BP_Sun.DefaultSceneRoot` (`self.Sun`)))) (`self.DistFromSun`))
    ;[1 1 1] Check all planets
    (for _array_element _
      (if (<= (`KismetMathLibrary.Vector_Distance` (`SceneComponent.K2_GetComponentLocation` (`/Game/Blueprints/BP_Planet_Base.StaticMesh` _array_element)) NewLoc) (`self.DistBetweenPlanets`))
        (return false)))
    (return true)
    (else
      (return false))))

(fn `GetNewPlanetLocation`
  (returns (NewLoc :type "Vector Structure"))
  (locals (NewLocation :type "Vector Structure" :default (0.0 0.0 0.0)))
  (bind _size (`self.Size`))
  (bind _returnvalue (* _size -0.5))
  (bind _returnvalue_2 (* _size 0.5))
  (bind _output_get (set `local.NewLocation` (`KismetMathLibrary.MakeVector` (`KismetMathLibrary.RandomFloatInRange` _returnvalue _returnvalue_2) (`KismetMathLibrary.RandomFloatInRange` _returnvalue _returnvalue_2) (`KismetMathLibrary.RandomFloatInRange` _returnvalue _returnvalue_2)) :!label _label))
  (bind _isokay (`self.CheckNewPlanetLocation` _output_get))
  (while (not _isokay)
    (goto _label))
  (return _output_get))

(fn `GetSoftCapSpeedMod`
  (params (Pos :type "Vector Structure") (Dir :type "Vector Structure"))
  (returns (SpeedMod :type "Float (double-precision)"))
  (bind _size (`self.Size`))
  (bind _returnvalue (`SceneComponent.K2_GetComponentLocation` (`self.DefaultSceneRoot`)))
  (bind _returnvalue_2 (`KismetMathLibrary.Vector_Distance` _returnvalue Pos))
  (bind _returnvalue_3 (`KismetMathLibrary.Dot_VectorVector` (`KismetMathLibrary.Normal` Dir) (`KismetMathLibrary.Normal` (- Pos _returnvalue))))
  (if (<= _returnvalue_2 _size)
    ;[1 1 1] Not in softcap
    (return 1.0)
    (else
      ;[1 1 1] Do 1.0f - (dotprod of dir and rootToPlayer) * distance into softcap range
      (if (<= _returnvalue_3 0.0)
        ;[1 1 1] Inbound player
        (return 1.0)
        (else
          (return (`KismetMathLibrary.FMax` (- 1.0 (/ (- _returnvalue_2 _size) (`self.SoftCapRange`))) (- 1.0 _returnvalue_3))))))))

(fn `SpawnPlanet`
  (returns (NewPlanet :type "/Game/Blueprints/BP_Planet_Base Object Reference"))
  (bind _possibleplanettypes (`self.PossiblePlanetTypes`))
  (bind _newloc (`self.GetNewPlanetLocation`))
  (bind _returnvalue (`|SpawnActorFromClass` (`|GetArrayItem` _possibleplanettypes (`KismetMathLibrary.RandomInteger` (- (`KismetArrayLibrary.Array_Length` _possibleplanettypes) 1))) (`KismetMathLibrary.MakeTransform` _newloc) "Undefined" "OverrideRootScale" null null))
  (return _returnvalue))

(fn `UserConstructionScript`)