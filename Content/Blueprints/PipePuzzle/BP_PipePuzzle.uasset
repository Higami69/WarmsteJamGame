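; Pipe puzzle board that spawns pipe pieces with random rotations and tracks whether they connect start to end.
; On BeginPlay it random-walks a solution path, using a reachability search to reject self-blocking steps, then spawns straight, bent or junction pieces along it.
; While active, Tick line-traces from the player's mesh to highlight a piece.
; TryCompletePuzzle, marked TODO for a button hookup, searches connected openings to set IsSolved.
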(event `self.ReceiveBeginPlay`
  ;[1 1 1] BeginPlay: Generate a board
  (`self.GenerateBoard`)
  (bind _asplayer (cast `/Game/Blueprints/Player` (`Controller.K2_GetPawn` (`GameplayStatics.GetPlayerController` 0))))
  (set `self.Player` _asplayer))

(event `self.ReceiveTick`
  (params (DeltaSeconds :type "Float (single-precision)"))
  ;[1 1 1] Check if there is a piece selected
  (if (and (`self.IsActive`) (not (`self.IsSolved`)))
    (`self.CheckPieceSelection`)))

(event `TryCompletePuzzle`
  ;[1 1 1] TryCompletePuzzle: TODO CALL FROM THE BUTTON
  (bind _wassolved (`self.CheckBoardWin`))
  (if _wassolved
    (set `self.IsSolved` true)))

(fn `CheckBoardWin`
  (returns (WasSolved :type Boolean))
  (locals (CheckedIdxs :type "Array of Integer") (IdxsToCheck :type "Array of Integer") (CurrIdx :type Integer) (CurrDir :type "/Game/Blueprints/PipePuzzle/DirVar Enum") (CurrDirs :type "Array of /Game/Blueprints/PipePuzzle/DirVar Enum"))
  (bind _curridx (`local.CurrIdx`))
  (bind _checkedidxs (`local.CheckedIdxs`))
  (bind _curridx_2 (`local.CurrIdx`))
  (bind _curridx_3 (`local.CurrIdx`))
  (bind _width (`self.Width`))
  (bind _idxstocheck (`local.IdxsToCheck`))
  (bind _idxstocheck_2 (`local.IdxsToCheck`))
  (bind _idxstocheck_3 (`local.IdxsToCheck`))
  (bind _returnvalue (- _curridx _width))
  (bind _returnvalue_2 (- _curridx_3 1))
  (bind _returnvalue_3 (+ _curridx _width))
  (bind _returnvalue_4 (+ _curridx_3 1))
  ;[1 1 1] Note: Bent are by default Up & Right, Straight Up & Down, Threeway All but Left
  (`KismetArrayLibrary.Array_Add` _idxstocheck (`self.StartIdx`))
  (while (> (`KismetArrayLibrary.Array_Length` _idxstocheck) 0)
    (bind _output_get (set `local.CurrIdx` (`|GetArrayItem` _idxstocheck_3)))
    (`KismetArrayLibrary.Array_RemoveItem` _idxstocheck_3 _output_get)
    (bind _returnvalue_5 (`KismetArrayLibrary.Array_Add` (`local.CheckedIdxs`) _output_get))
    (if (== (`local.CurrIdx`) (`self.EndIdx`))
      (return true)
      (else
        (`|ExecutionSequence`
          (:`then_0`
            (bind _dirs (`/Game/Blueprints/PipePuzzle/BP_PipePiece.GetActualDirs` (`|GetArrayItem` (`self.Pieces`) _returnvalue_5)))
            (set `local.CurrDirs` _dirs))
          (:`then_1`
            ;[1 1 1] Go over all dirs, check if we can go to that idx
            (for _array_element (`local.CurrDirs`)
              ;[1 1 1] Can we go there?
              (switch `/Game/Blueprints/PipePuzzle/DirVar` _array_element
                (:`NewEnumerator0`
                  (if (`self.CanGoUp` _curridx_2)
                    ;[1 1 1] Have we not checked this idx already?
                    (if (not (`KismetArrayLibrary.Array_Contains` _checkedidxs _returnvalue))
                      ;[1 1 1] Can the target receive us?
                      (bind _dirs_2 (`/Game/Blueprints/PipePuzzle/BP_PipePiece.GetActualDirs` (`|GetArrayItem` (`self.Pieces`) _returnvalue)))
                      (if (`KismetArrayLibrary.Array_Contains` _dirs_2 "NewEnumerator2")
                        ;[1 1 1] Add to idxs to search
                        (`KismetArrayLibrary.Array_Add` _idxstocheck_2 _returnvalue)))))
                (:`NewEnumerator1`
                  (if (`self.CanGoLeft` _curridx_2)
                    (if (not (`KismetArrayLibrary.Array_Contains` _checkedidxs _returnvalue_2))
                      (bind _dirs_3 (`/Game/Blueprints/PipePuzzle/BP_PipePiece.GetActualDirs` (`|GetArrayItem` (`self.Pieces`) _returnvalue_2)))
                      (if (`KismetArrayLibrary.Array_Contains` _dirs_3 "NewEnumerator3")
                        (`KismetArrayLibrary.Array_Add` _idxstocheck_2 _returnvalue_2)))))
                (:`NewEnumerator2`
                  (if (`self.CanGoDown` _curridx_2)
                    (if (not (`KismetArrayLibrary.Array_Contains` _checkedidxs _returnvalue_3))
                      (bind _dirs_4 (`/Game/Blueprints/PipePuzzle/BP_PipePiece.GetActualDirs` (`|GetArrayItem` (`self.Pieces`) _returnvalue_3)))
                      (if (`KismetArrayLibrary.Array_Contains` _dirs_4 "NewEnumerator0")
                        (`KismetArrayLibrary.Array_Add` _idxstocheck_2 _returnvalue_3)))))
                (:`NewEnumerator3`
                  (if (`self.CanGoRight` _curridx_2)
                    (if (not (`KismetArrayLibrary.Array_Contains` _checkedidxs _returnvalue_4))
                      (bind _dirs_5 (`/Game/Blueprints/PipePuzzle/BP_PipePiece.GetActualDirs` (`|GetArrayItem` (`self.Pieces`) _returnvalue_4)))
                      (if (`KismetArrayLibrary.Array_Contains` _dirs_5 "NewEnumerator1")
                        (`KismetArrayLibrary.Array_Add` _idxstocheck_2 _returnvalue_4))))))))))))
  (return false))

(fn `CheckPieceSelection`
  (bind _mesh (`/Game/Blueprints/Player.Mesh` (`self.Player`)))
  (bind _returnvalue (`SceneComponent.K2_GetComponentLocation` _mesh))
  ;[1 1 1] Unselect all pipes
  (for _array_element (`self.Pieces`)
    (`/Game/Blueprints/PipePuzzle/BP_PipePiece.SetSelected` _array_element false))
  (bind _outhit (`KismetSystemLibrary.LineTraceSingleForObjects` _returnvalue (+ _returnvalue (* (`SceneComponent.GetForwardVector` _mesh) 1000.0)) (`|MakeArray` "ObjectTypeQuery1" :!type "EObjectTypeQuery Enum")))
  (bind _asbp_pipe_piece (cast `/Game/Blueprints/PipePuzzle/BP_PipePiece` (`.HitActor` (`GameplayStatics.BreakHitResult` _outhit))))
  (`/Game/Blueprints/PipePuzzle/BP_PipePiece.SetSelected` _asbp_pipe_piece true))

(fn `DidSolutionBlockItself`
  (params (CurrSol :type "Array of /Game/Blueprints/PipePuzzle/SolutionVar Structure"))
  (returns (DidBlock :type Boolean))
  (locals (BlockedIdxs :type "Array of /Game/Blueprints/PipePuzzle/BoolArray Structure") (StartingIdx :type Integer) (IdxsToSearch :type "Array of Integer") (CanReach :type Boolean) (CurrIdx :type Integer))
  (bind _idxstosearch (`local.IdxsToSearch`))
  (bind _curridx (`local.CurrIdx`))
  (bind _width (`self.Width`))
  (bind _curridx_2 (`local.CurrIdx`))
  (bind _width_2 (`self.Width`))
  (bind _blockedidxs (`local.BlockedIdxs`))
  (bind _idxstosearch_2 (`local.IdxsToSearch`))
  (bind _blockedidxs_2 (`local.BlockedIdxs`))
  (bind _blockedidxs_3 (`local.BlockedIdxs`))
  (bind _idxstosearch_3 (`local.IdxsToSearch`))
  (bind _returnvalue (- _curridx_2 _width_2))
  (bind _returnvalue_2 (- _curridx 1))
  (bind _returnvalue_3 (+ _curridx_2 _width_2))
  (bind _returnvalue_4 (+ _curridx 1))
  (bind _output_targidx (break `/Game/Blueprints/PipePuzzle/SolutionVar` (`|GetArrayItem` CurrSol (`KismetArrayLibrary.Array_LastIndex` CurrSol))))
  (bind _output_row (break `/Game/Blueprints/PipePuzzle/BoolArray` (`|GetArrayItem` _blockedidxs_3 (`KismetArrayLibrary.Array_LastIndex` _blockedidxs_3))))
  (`|ExecutionSequence`
    (:`then_0`
      ;[1 1 1] Fill BlockedIdxs
      (for _index (range (+ (`self.Height`) 1))
        (`KismetArrayLibrary.Array_Add` _blockedidxs_3 (make `/Game/Blueprints/PipePuzzle/BoolArray` (`|MakeArray` false)))
        (for _index_2 (range (+ _width 1))
          (for _array_element CurrSol
            (if (== (+ (* _index _width) _index_2) (`.SrcIdx_8_EC72F0D14F11DB8D01E8A39EDD2AD27D` (break `/Game/Blueprints/PipePuzzle/SolutionVar` _array_element)))
              (`KismetArrayLibrary.Array_Add` _output_row true)
              (break)))
          (`KismetArrayLibrary.Array_Add` _output_row))))
    (:`then_1`
      ;[1 1 1] Check if we should continue loop
      (bind _output_get (set `local.StartingIdx` _output_targidx))
      (`KismetArrayLibrary.Array_Add` _idxstosearch _output_get)
      (while (> (`KismetArrayLibrary.Array_Length` _idxstosearch) 0)
        (if (== (`|GetArrayItem` _idxstosearch_3) (`self.EndIdx`))
          (set `local.CanReach` true)
          (`KismetArrayLibrary.Array_Clear` (`local.IdxsToSearch`)) ; End while loop
          (else
            (bind _output_get_2 (set `local.CurrIdx` (`|GetArrayItem` _idxstosearch_3 (`KismetArrayLibrary.Array_LastIndex` _idxstosearch_3))))
            (`KismetArrayLibrary.Array_RemoveItem` (`local.IdxsToSearch`) _output_get_2)
            (`|ExecutionSequence`
              (:`then_0`
                ;[1 1 1] Add new idxs to idxs to search
                (if (`self.CanGoUp` 0)
                  (if (`self.IsIdxFree` _blockedidxs_2 _returnvalue)
                    (bind _returnvalue_5 (`KismetArrayLibrary.Array_Add` _idxstosearch_2 _returnvalue))
                    (`self.SetIdxBlocked` _blockedidxs _returnvalue_5))))
              (:`then_1`
                (if (`self.CanGoDown` 0)
                  (if (`self.IsIdxFree` _blockedidxs_2 _returnvalue_3)
                    (bind _returnvalue_6 (`KismetArrayLibrary.Array_Add` _idxstosearch_2 _returnvalue_3))
                    (`self.SetIdxBlocked` _blockedidxs _returnvalue_6))))
              (:`then_2`
                (if (`self.CanGoLeft` 0)
                  (if (`self.IsIdxFree` _blockedidxs_2 _returnvalue_2)
                    (bind _returnvalue_7 (`KismetArrayLibrary.Array_Add` _idxstosearch_2 _returnvalue_2))
                    (`self.SetIdxBlocked` _blockedidxs _returnvalue_7))))
              (:`then_3`
                (if (`self.CanGoRight` 0)
                  (if (`self.IsIdxFree` _blockedidxs_2 _returnvalue_4)
                    (bind _returnvalue_8 (`KismetArrayLibrary.Array_Add` _idxstosearch_2 _returnvalue_4))
                    (`self.SetIdxBlocked` _blockedidxs _returnvalue_8))))))))
      (return (not (`local.CanReach`))))))

(fn `GenerateBoard`
  (locals (Solution :type "Array of /Game/Blueprints/PipePuzzle/SolutionVar Structure") (SolutionFound :type Boolean) (Cols :type "Array of /Game/Blueprints/PipePuzzle/BoolArray Structure"))
  (bind _solutionvar (make `/Game/Blueprints/PipePuzzle/SolutionVar` 0))
  (bind _solution (`local.Solution`))
  (bind _solution_2 (`local.Solution`))
  (bind _solution_3 (`local.Solution`))
  (`|ExecutionSequence`
    (:`then_0`
      ;[1 1 1] Generate A Solution
      (while (not (`local.SolutionFound`))
        (`self.GenerateRandomStep` _solution_3)
        (bind _didblock (`self.DidSolutionBlockItself` _solution_3))
        ;;[1 1 1] Check if we reached the end
        (if _didblock
          (`KismetArrayLibrary.Array_RemoveItem` _solution_2 (`|GetArrayItem` _solution (`KismetArrayLibrary.Array_LastIndex` _solution)))
          (else
            (`KismetArrayLibrary.Array_Add` _solution_2 _solutionvar)
            (set `local.SolutionFound` (== (`.TargIdx_2_9E88DA2D4018073482F610B7CD988F3C` (break `/Game/Blueprints/PipePuzzle/SolutionVar` _solutionvar)) (`self.EndIdx`)))))))
    (:`then_1`
      ;[1 1 1] Fill out grid
      (for _index (range (* (`self.Height`) (`self.Width`)))
        ;[1 1 1] Generate pipes
        (for _array_element (`local.Solution`)
          (bind (_targidx _dir _srcidx _srcdir) (break `/Game/Blueprints/PipePuzzle/SolutionVar` _array_element))
          (if (== _index _srcidx)
            (switch `/Game/Blueprints/PipePuzzle/DirVar` _dir
              (:`NewEnumerator0`
                (switch `/Game/Blueprints/PipePuzzle/DirVar` _srcdir
                  (:`NewEnumerator0`
                    (`self.SpawnStraightPipeAtIdx` _srcidx :!label _label))
                  (:`NewEnumerator1`
                    (`self.SpawnBentPipeAtIdx` _srcidx :!label _label_2))
                  (:`NewEnumerator2`
                    (goto _label))
                  (:`NewEnumerator3`
                    (goto _label_2))))
              (:`NewEnumerator1`
                (switch `/Game/Blueprints/PipePuzzle/DirVar` _srcdir
                  (:`NewEnumerator0`
                    (goto _label_2))
                  (:`NewEnumerator1`
                    (goto _label))
                  (:`NewEnumerator2`
                    (goto _label_2))
                  (:`NewEnumerator3`
                    (goto _label))))
              (:`NewEnumerator2`
                (switch `/Game/Blueprints/PipePuzzle/DirVar` _srcdir
                  (:`NewEnumerator0`
                    (goto _label))
                  (:`NewEnumerator1`
                    (goto _label_2))
                  (:`NewEnumerator2`
                    (goto _label))
                  (:`NewEnumerator3`
                    (goto _label_2))))
              (:`NewEnumerator3`
                (switch `/Game/Blueprints/PipePuzzle/DirVar` _srcdir
                  (:`NewEnumerator0`
                    (goto _label_2))
                  (:`NewEnumerator1`
                    (goto _label))
                  (:`NewEnumerator2`
                    (goto _label_2))
                  (:`NewEnumerator3`
                    (goto _label)))))))))
    (:`then_2`
      ;[1 1 1] Randomly Rotate All Pipes
      (for _array_element_2 (`self.Pieces`)
        (`/Game/Blueprints/PipePuzzle/BP_PipePiece.SetNewRotation` :`self` _array_element_2 :`NewRot` (`KismetMathLibrary.RandomInteger` 3))))))

(fn `GenerateRandomStep`
  (params (CurrSolution :type "Array of /Game/Blueprints/PipePuzzle/SolutionVar Structure (by ref)"))
  (locals (NewDir :type "/Game/Blueprints/PipePuzzle/DirVar Enum") (NewIdx :type Integer))
  (bind _width (`self.Width`))
  (bind _width_2 (`self.Width`))
  (bind (_output_targidx _output_dir) (break `/Game/Blueprints/PipePuzzle/SolutionVar` (`|GetArrayItem` CurrSolution (`KismetArrayLibrary.Array_LastIndex` CurrSolution))))
  (bind _returnvalue (/ _output_targidx (`self.Width`)))
  (bind _returnvalue_2 (mod _output_targidx _width))
  (bind _returnvalue_3 (cast `/Game/Blueprints/PipePuzzle/DirVar` (`KismetMathLibrary.Conv_IntToByte` (`KismetMathLibrary.RandomInteger` (`KismetMathLibrary.Conv_ByteToInt` (enumliteral `/Game/Blueprints/PipePuzzle/DirVar` "NewEnumerator3"))))))
  ;[1 1 1] Get new direction that is valid
  (bind _output_get (set `local.NewDir` _returnvalue_3 :!label _label))
  (if (`|EnumInequality` _output_dir _returnvalue_3)
    (switch `/Game/Blueprints/PipePuzzle/DirVar` _output_get
      (:`NewEnumerator0`
        ;[1 1 1] Check execution
        (if (< _returnvalue (`self.Height`))
          ;[1 1 1] Set new target idx
          (set `local.NewIdx` (+ _output_targidx _width_2))
          (else
            (goto _label))))
      (:`NewEnumerator1`
        (if (> _returnvalue_2 0)
          (set `local.NewIdx` (- _output_targidx 1))
          (else
            (goto _label))))
      (:`NewEnumerator2`
        (if (> _returnvalue 0)
          (set `local.NewIdx` (- _output_targidx _width_2))
          (else
            (goto _label))))
      (:`NewEnumerator3`
        (if (< _returnvalue_2 (- _width 1))
          (set `local.NewIdx` (+ _output_targidx 1))
          (else
            (goto _label)))))
    ;[1 1 1] jesus christ
    (`KismetArrayLibrary.Array_Add` CurrSolution (make `/Game/Blueprints/PipePuzzle/SolutionVar` (`local.NewIdx`) (`local.NewDir`) _output_targidx _output_dir))
    (else
      (goto _label))))

(fn `GetLocationAtIdx`
  (params (Idx :type Integer))
  (returns (Location :type "Vector Structure"))
  (bind _width (`self.Width`))
  (return (+ (`KismetMathLibrary.MakeVector` (* (`self.Height`) (`KismetMathLibrary.Conv_IntToDouble` (/ Idx _width))) (* (`self.Width`) (`KismetMathLibrary.Conv_IntToDouble` (mod Idx _width)))) (`SceneComponent.K2_GetComponentLocation` (`self.DefaultSceneRoot`)))))

(fn `SetIdxBlocked`
  (params (BlockedIdxs :type "Array of /Game/Blueprints/PipePuzzle/BoolArray Structure (by ref)") (Idx :type "Integer (by ref)"))
  (bind _width (`self.Width`))
  (bind _output_row (break `/Game/Blueprints/PipePuzzle/BoolArray` (`|GetArrayItem` BlockedIdxs (/ Idx _width))))
  (`KismetArrayLibrary.Array_Set` _output_row (mod Idx _width) true))

(fn `SpawnBentPipeAtIdx`
  (params (Idx :type Integer))
  (switch `int` (`KismetMathLibrary.RandomInteger` 3)
    (:`0`
      (`self.SpawnPipeOfClassAtIdx` Idx "/Game/Blueprints/PipePuzzle/BP_PipePiece_Bent.BP_PipePiece_Bent_C" :!label _label))
    (:`1`
      (goto _label))
    (:`2`
      (`self.SpawnPipeOfClassAtIdx` Idx "/Game/Blueprints/PipePuzzle/BP_PipePiece_Threeway.BP_PipePiece_Threeway_C"))
    (:`3`
      (`self.SpawnPipeOfClassAtIdx` Idx "/Game/Blueprints/PipePuzzle/BP_PipePiece_FourWay.BP_PipePiece_FourWay_C"))))

(fn `SpawnPipeOfClassAtIdx`
  (params (Idx :type Integer) (Class :type "/Game/Blueprints/PipePuzzle/BP_PipePiece Class Reference"))
  (bind _location (`self.GetLocationAtIdx` Idx))
  (bind _returnvalue (`|SpawnActorFromClass` Class (`KismetMathLibrary.MakeTransform` _location) "Undefined" "OverrideRootScale" null null))
  (`KismetArrayLibrary.Array_Add` (`self.Pieces`) _returnvalue))

(fn `SpawnStraightPipeAtIdx`
  (params (Idx :type Integer))
  (switch `int` (`KismetMathLibrary.RandomInteger` 3)
    (:`0`
      (`self.SpawnPipeOfClassAtIdx` Idx "/Game/Blueprints/PipePuzzle/BP_PipePiece_Straight.BP_PipePiece_Straight_C" :!label _label))
    (:`1`
      (goto _label))
    (:`2`
      (`self.SpawnPipeOfClassAtIdx` Idx "/Game/Blueprints/PipePuzzle/BP_PipePiece_Threeway.BP_PipePiece_Threeway_C"))
    (:`3`
      (`self.SpawnPipeOfClassAtIdx` Idx "/Game/Blueprints/PipePuzzle/BP_PipePiece_FourWay.BP_PipePiece_FourWay_C"))))

(fn `UserConstructionScript`)