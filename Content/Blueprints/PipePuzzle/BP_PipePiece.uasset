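; BP_PipePiece is a rotatable piece for the pipe puzzle, with a list of possible directions.
; SetNewRotation wraps the input to four quarter-turn steps, stores it as Rot and applies that yaw combined with the parent's rotation.
; GetActualDirs switches on each possible direction and Rot into four shared add nodes, though all four add Up as written.
; SetSelected is an empty stub.
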(event `SetNewRotation`
  (params (NewRot :type Integer) (ParentRot :type "Rotator Structure"))
  (bind _output_get (set `self.Rot` (mod NewRot 4)))
  (`SceneComponent.K2_SetWorldRotation` (`self.DefaultSceneRoot`) (`KismetMathLibrary.ComposeRotators` ParentRot (`KismetMathLibrary.MakeRotator` 0.0 0.0 (* _output_get 90.0))) false false))

(fn `GetActualDirs`
  (returns (Dirs :type "Array of /Game/Blueprints/PipePuzzle/DirVar Enum"))
  (locals (NewDirs :type "Array of /Game/Blueprints/PipePuzzle/DirVar Enum"))
  (bind _rot (`self.Rot`))
  (bind _newdirs (`local.NewDirs`))
  (for _array_element (`self.PossibleDirs`)
    (switch `/Game/Blueprints/PipePuzzle/DirVar` _array_element
      (:`NewEnumerator0`
        (switch `int` _rot
          (:`0`
            (`KismetArrayLibrary.Array_Add` _newdirs "NewEnumerator0" :!label _label))
          (:`1`
            (`KismetArrayLibrary.Array_Add` _newdirs "NewEnumerator0" :!label _label_2))
          (:`2`
            (`KismetArrayLibrary.Array_Add` _newdirs "NewEnumerator0" :!label _label_3))
          (:`3`
            (`KismetArrayLibrary.Array_Add` _newdirs "NewEnumerator0" :!label _label_4))))
      (:`NewEnumerator1`
        (switch `int` _rot
          (:`0`
            (goto _label_4))
          (:`1`
            (goto _label))
          (:`2`
            (goto _label_2))
          (:`3`
            (goto _label_3))))
      (:`NewEnumerator2`
        (switch `int` _rot
          (:`0`
            (goto _label_3))
          (:`1`
            (goto _label_4))
          (:`2`
            (goto _label))
          (:`3`
            (goto _label_2))))
      (:`NewEnumerator3`
        (switch `int` _rot
          (:`0`
            (goto _label_2))
          (:`1`
            (goto _label_3))
          (:`2`
            (goto _label_4))
          (:`3`
            (goto _label))))))
  (return (`local.NewDirs`)))

(fn `SetSelected`
  (params (Selected :type Boolean)))

(fn `UserConstructionScript`)